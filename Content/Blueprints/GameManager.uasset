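; GameManager lists saved custom maps in the main HUD, then builds the selected map and spawns a TwinStickPawn.
; GetSave caches the SaveCustomMap object, loading its save slot or creating and saving a new one.
; ShowAllLevels passes the saved map names to MainHud, whose level-select event looks up the chosen map.
; OpenLevel builds a map by adding a static mesh component at each stored tile position.
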(event Custom|PrintNames
  (params (LevelName :type Integer))
  (CallFunction|OpenLevel (.Value (Utilities|Map|Find (Variables|Default|GetMap%20Level) LevelName)))
  (CallFunction|SpawCharacter))

(event EventBeginPlay
  (CallFunction|CreateMainWidget (delegate Custom|PrintNames))
  (CallFunction|ShowAllLevels))

(fn ConstructionScript)

(fn GetSave
  (Utilities|IsValid (Variables|Default|GetAs%20Save%20Custom%20Map)
    (:Is%20Valid
      _)
    (:Is%20Not%20Valid
      (bind _returnvalue (SaveGame|LoadGamefromSlot "SaveCustomMap"))
      (Utilities|IsValid _returnvalue
        (:Is%20Valid
          (bind _assave_custom_map (Utilities|Casting|CastToSaveCustomMap _returnvalue))
          (Variables|Default|SetAs%20Save%20Custom%20Map _assave_custom_map))
        (:Is%20Not%20Valid
          (bind _returnvalue_2 (SaveGame|CreateSaveGameObject "/Game/Blueprints/SaveCustomMap.SaveCustomMap_C"))
          (SaveGame|SaveGametoSlot _returnvalue_2 "SaveCustomMap")
          (Variables|Default|SetAs%20Save%20Custom%20Map _returnvalue_2)))))
  (return (Variables|Default|GetAs%20Save%20Custom%20Map)))

(fn ShowAllLevels
  (bind _as_save_custom_map (CallFunction|GetSave))
  (Variables|Default|SetMap%20Level (Variables|/Game/Blueprints/SaveCustomMap.SaveCustomMap_C|GetMapLevel _as_save_custom_map))
  (Default|ShowAllLevels (Variables|Default|GetNewVar_0) (CallFunction|ParseLevelList (Variables|/Game/Blueprints/SaveCustomMap.SaveCustomMap_C|GetMapLevel _as_save_custom_map))))

(fn CreateMainWidget
  (params (Event :type Delegate%20%28by%20ref%29))
  (bind _returnvalue (UserInterface|CreateWidget "/Game/Widgets/MainHud.MainHud_C"))
  (UserInterface|Viewport|AddtoViewport _returnvalue 0)
  (bind _output_get (Variables|Default|SetNewVar_0 _returnvalue))
  (EventDispatchers|BindEventtoLevelSelect _output_get Event))

(fn ParseLevelList
  (params (NewParam :type Map%20of%20Integers%20to%20Structs))
  (bind _mapname (LocalVariables|GetMapName))
  (bind _keys (Utilities|Map|Keys NewParam))
  (for _array_element _keys
    (Utilities|Map|Add _mapname _array_element (Utilities|Struct|BreakLevelInformation (.Value (Utilities|Map|Find NewParam _array_element)))))
  (return _mapname))

(fn OpenLevel
  (params (NewParam :type Level%20Information%20Structure))
  (for _array_element (Utilities|Struct|BreakLevelInformation NewParam)
    (AddComponent|AddStaticMeshComponent false (Math|Transform|MakeTransform _array_element "0, 0, 0" "1,1,1"))))

(fn SpawCharacter
  (bind _returnvalue (Game|SpawnActorfromClass "/Game/TwinStickBP/Blueprints/TwinStickPawn.TwinStickPawn_C" (Math|Transform|MakeTransform "0, 0, 0" "0, 0, 0" "1,1,1") "Undefined" 0 0))
  (Variables|Default|SetPlayerCustom _returnvalue))