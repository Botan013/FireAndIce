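; Tile path editor actor that builds a level one platform at a time from a starting tile.
; Four directional widget buttons each add a static mesh tile at a grid offset, then move around it, hiding the one pointing back.
; Tick eases an overhead camera toward the newest tile.
; An editor widget reloads the level on Clear and spawns and possesses a TwinStickPawn on Start; Save is an empty stub.
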(event OnClicked(WidgetUp)
  (params (TouchedComponent :type Primitive%20Component%20Object%20Reference) (ButtonPressed :type Key%20Structure :default "None"))
  (CallFunction|ButtononClicked 1))

(event OnClicked(WidgetRight)
  (params (TouchedComponent :type Primitive%20Component%20Object%20Reference) (ButtonPressed :type Key%20Structure :default "None"))
  (CallFunction|ButtononClicked 2))

(event OnClicked(WidgetLeft)
  (params (TouchedComponent :type Primitive%20Component%20Object%20Reference) (ButtonPressed :type Key%20Structure :default "None"))
  (CallFunction|ButtononClicked))

(event OnClicked(WidgetDown)
  (params (TouchedComponent :type Primitive%20Component%20Object%20Reference) (ButtonPressed :type Key%20Structure :default "None"))
  (CallFunction|ButtononClicked 3))

(event Custom|ButtonOnClicked
  (params (Index :type Integer))
  (bind _nextposition (CallFunction|GetSpawnLocation Index))
  (CallFunction|SpawnPlatform _nextposition)
  (Variables|Default|SetPreviosPosition (Math|Integer|%(Integer) (+ Index 2) 4))
  (CallFunction|SetButtonPosition))

(event EventBeginPlay
  (CallFunction|CreateRedactorWidget)
  (CallFunction|CreateRedactorButtons (delegate Custom|ButtonOnClicked))
  (CallFunction|SpawnPlatform)
  (CallFunction|SetButtonPosition))

(event EventTick
  (params (DeltaSeconds :type Float%20%28single-precision%29))
  (bind _camera (Variables|Default|GetCamera))
  (bind _currentposition (Variables|Default|GetCurrentPosition))
  (bind _returnvalue (Transformation|GetWorldLocation _camera))
  (bind _returnvalue_2 (Math|Interpolation|VInterpTo _returnvalue _currentposition DeltaSeconds 1.0))
  (Transformation|SetWorldLocation _camera (Math|Vector|MakeVector (.x _returnvalue_2) (.y _returnvalue_2) 2.4e+03) false false))

(event Custom|CreateRedactorWidget
  (bind _returnvalue (UserInterface|CreateWidget "/Game/Widgets/RedactorWidget.RedactorWidget_C"))
  (UserInterface|Viewport|AddtoViewport _returnvalue 0)
  (EventDispatchers|AssignOnClicked (Variables|/Game/Widgets/RedactorWidget.RedactorWidget_C|GetClear _returnvalue) (delegate Custom|OnClicked_Event_2))
  (EventDispatchers|AssignOnClicked (Variables|/Game/Widgets/RedactorWidget.RedactorWidget_C|GetStart _returnvalue) (delegate Custom|OnClicked_Event_1))
  (EventDispatchers|AssignOnClicked (Variables|/Game/Widgets/RedactorWidget.RedactorWidget_C|GetSave _returnvalue) (delegate Custom|OnClicked_Event_0)))

(event Custom|OnClicked_Event_0)

(event Custom|OnClicked_Event_1
  (CallFunction|SpawnFireandIce))

(event Custom|OnClicked_Event_2
  (Game|OpenLevel(byName) "Redactor"))

(fn ConstructionScript)

(fn CreateRedactorButtons
  (params (Event :type Delegate%20%28by%20ref%29))
  (bind _widgetdown (Variables|Default|GetWidgetDown))
  (bind _mapstructures (Variables|Default|GetMapStructures))
  (Utilities|FlowControl|Sequence
    (:then_0
      (bind _asbutton (Utilities|Casting|CastToButton (UserInterface|GetUserWidgetObject _widgetdown)))
      (Variables|/Game/Widgets/Button.Button_C|SetIndex _asbutton 3)
      (EventDispatchers|BindEventtoOnClicked _asbutton Event)
      (Rendering|Components|TextRender|SetText (Variables|/Game/Widgets/Button.Button_C|GetTextBlock_47 _asbutton) "Down"))
    (:then_1
      (bind _asbutton_2 (Utilities|Casting|CastToButton (UserInterface|GetUserWidgetObject (Variables|Default|GetWidgetLeft))))
      (Variables|/Game/Widgets/Button.Button_C|SetIndex _asbutton_2 0)
      (EventDispatchers|BindEventtoOnClicked _asbutton_2 Event)
      (Rendering|Components|TextRender|SetText (Variables|/Game/Widgets/Button.Button_C|GetTextBlock_47 _asbutton_2) "Left"))
    (:then_2
      (bind _asbutton_3 (Utilities|Casting|CastToButton (UserInterface|GetUserWidgetObject (Variables|Default|GetWidgetUp))))
      (Variables|/Game/Widgets/Button.Button_C|SetIndex _asbutton_3 1)
      (EventDispatchers|BindEventtoOnClicked _asbutton_3 Event)
      (Rendering|Components|TextRender|SetText (Variables|/Game/Widgets/Button.Button_C|GetTextBlock_47 _asbutton_3) "Up"))
    (:then_3
      (bind _asbutton_4 (Utilities|Casting|CastToButton (UserInterface|GetUserWidgetObject (Variables|Default|GetWidgetRight))))
      (Variables|/Game/Widgets/Button.Button_C|SetIndex _asbutton_4 2)
      (EventDispatchers|BindEventtoOnClicked _asbutton_4 Event)
      (Rendering|Components|TextRender|SetText (Variables|/Game/Widgets/Button.Button_C|GetTextBlock_47 _asbutton_4) "Right"))
    (:then_4
      (Utilities|Map|Add _mapstructures 3 (Utilities|Struct|MakeButtonInfo "(X=0.000000,Y=-1.000000)" _widgetdown))
      (Utilities|Map|Add _mapstructures 1 (Utilities|Struct|MakeButtonInfo "(X=0.000000,Y=1.000000)" (Variables|Default|GetWidgetUp)))
      (Utilities|Map|Add _mapstructures 2 (Utilities|Struct|MakeButtonInfo "(X=1.000000,Y=0.000000)" (Variables|Default|GetWidgetRight)))
      (Utilities|Map|Add _mapstructures 0 (Utilities|Struct|MakeButtonInfo "(X=-1.000000,Y=0.000000)" (Variables|Default|GetWidgetLeft))))))

(fn GetSpawnLocation
  (params (Index :type Integer))
  (return (.Offset (Utilities|Struct|BreakButtonInfo (.Value (Utilities|Map|Find (Variables|Default|GetMapStructures) Index))))))

(fn SpawnPlatform
  (params (SpawnPosition :type Vector%202D%20Structure))
  (bind _output_get (Variables|Default|SetCurrentPosition (+ (Math|Conversions|ToVector(Vector2D) (* SpawnPosition (Variables|Default|GetTileSize))) (Variables|Default|GetCurrentPosition))))
  (bind _returnvalue (AddComponent|AddStaticMeshComponent false (Math|Transform|MakeTransform _output_get)))
  (Utilities|Array|Add (Variables|Default|GetMeshMaasiv) _returnvalue))

(fn SetButtonPosition
  (bind _previosposition (Variables|Default|GetPreviosPosition))
  (bind _tilesize (Variables|Default|GetTileSize))
  (bind _returnvalue (/ _tilesize -2.0))
  (bind _output_get (LocalVariables|SetNewLocalVar_0 (Variables|Default|GetMapStructures)))
  (Rendering|SetVisibility (.RefButton (Utilities|Struct|BreakButtonInfo (.Value (Utilities|Map|Find _output_get _previosposition)))) false false)
  (Utilities|Map|Remove _output_get _previosposition)
  (bind _values (Utilities|Map|Values _output_get))
  (for _array_element _values
    (Rendering|SetVisibility (.RefButton (Utilities|Struct|BreakButtonInfo _array_element)) true false)
    (Transformation|SetWorldLocation (.RefButton (Utilities|Struct|BreakButtonInfo _array_element)) (- (+ (* (Math|Conversions|ToVector(Vector2D) (.Offset (Utilities|Struct|BreakButtonInfo _array_element))) (Variables|Default|GetTileSize)) (Variables|Default|GetCurrentPosition)) (Math|Vector|MakeVector _returnvalue _returnvalue 0.0)) false false)))

(fn SpawnFireandIce
  (bind _returnvalue (Game|SpawnActorfromClass "/Game/TwinStickBP/Blueprints/TwinStickPawn.TwinStickPawn_C" (Math|Transform|MakeTransform (Math|Conversions|ToVector(Float) (/ (Variables|Default|GetTileSize) 2.0))) "Undefined" 0 0))
  (Pawn|Possess (Game|GetPlayerController 0) _returnvalue))